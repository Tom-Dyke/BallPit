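; EndBox is an overlap actor that flags when the player character's mesh reaches an end area.
; On any actor overlap, it loops through its overlapping components looking for the mesh of player character 0.
; A match casts the player to BP_ThirdPersonCharacter, sets its MeshAtEnd flag and prints a debug message.
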(event EventBeginPlay)

(event Collision|EventActorBeginOverlap
  (params (OtherActor :type Actor%20Object%20Reference))
  (for _array_element (Class|Actor|GetOverlappingComponents self)
    (if (== (Variables|/Script/Engine.Character|GetMesh (Game|GetPlayerCharacter 0)) _array_element)
      (bind _asbp_third_person_character (Utilities|Casting|CastToBP_ThirdPersonCharacter (Game|GetPlayerCharacter 0)))
      (Variables|/Game/ThirdPerson/Blueprints/BP_ThirdPersonCharacter.BP_ThirdPersonCharacter_C|SetMeshAtEnd _asbp_third_person_character true)
      (Development|PrintString "Mesh At End"))))

(event EventTick
  (params (DeltaSeconds :type Float%20%28single-precision%29)))

(fn ConstructionScript)