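; Actor component that spawns a capped number of random, physics-simulated objects at a timed interval, using Tick with Delay and DoN.
; On the first spawn it copies the class list from MyGameInstance, printing a warning if empty.
; Rain mode drops randomly scaled objects across a hardcoded area; otherwise they launch from the owner with a fixed or randomized (Spread) impulse.
; Also defines a delayed for-each macro, unused in this graph.
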(event EventTick
  (params (DeltaSeconds :type Float%20%28single-precision%29))
  (bind _scale__max_ (Variables|Default|GetScale%20%28Max%29))
  (bind _scale__min_ (Variables|Default|GetScale%20%28Min%29))
  (bind _scale__max__2 (Variables|Default|GetScale%20%28Max%29))
  (bind _objects_to_spawn (Variables|Default|GetObjects%20to%20Spawn))
  (bind _objects_to_spawn_2 (Variables|Default|GetObjects%20to%20Spawn))
  (bind _scale__min__2 (Variables|Default|GetScale%20%28Min%29))
  (bind _returnvalue (Math|Random|RandomFloatinRange _scale__min__2 _scale__max_))
  (bind _returnvalue_2 (Math|Random|RandomFloatinRange _scale__min_ _scale__max__2))
  (Utilities|FlowControl|Delay (Variables|Default|GetDelay))
  (Utilities|FlowControl|DoN (Variables|Default|GetNumberOfObjects)
    (:Exit
      (Utilities|FlowControl|Sequence
        (:then_0
          (Utilities|FlowControl|DoOnce false
            (:Completed
              (bind _asmy_game_instance (Utilities|Casting|CastToMyGameInstance (Game|GetGameInstance)))
              (for _array_element (Variables|/Game/MyGameInstance.MyGameInstance_C|GetObjectsToSpawn _asmy_game_instance)
                (Utilities|Array|Add (Variables|Default|GetObjects%20to%20Spawn) _array_element)))))
        (:then_1
          (if (Variables|Default|GetRain)
            (if (Utilities|Array|IsEmpty _objects_to_spawn)
              (Development|PrintString "No Objects Found to Spawn, Please Load \"Start Game Level\", and play from there" :!label _label)
              (else
                (bind _returnvalue_3 (Game|SpawnActorfromClass (.OutItem (Utilities|Array|Random _objects_to_spawn)) (Math|Transform|MakeTransform (Math|Vector|MakeVector (Math|Random|RandomFloatinRange 1.1e+02 2.87e+03) (Math|Random|RandomFloatinRange 1.2e+02 3.38e+03) 7.2e+02) "0, 0, 0" (Math|Vector|MakeVector _returnvalue_2 _returnvalue_2 _returnvalue_2)) "Undefined" 0 0))
                (bind _staticmesh (Variables|/Game/Blueprints/ObjectSpawnSelection/SM_ObjectBlueprint.SM_ObjectBlueprint_C|GetStaticMesh _returnvalue_3)
                  (:then
                    (Physics|SetSimulatePhysics _staticmesh true))
                  (:else))))
            (elif (Utilities|Array|IsEmpty _objects_to_spawn_2)
              (goto _label)
              (else
                (bind _returnvalue_4 (Game|SpawnActorfromClass (.OutItem (Utilities|Array|Random _objects_to_spawn_2)) (Math|Transform|MakeTransform (.location (Transformation|GetActorTransform (Components|GetOwner self))) "0, 0, 0" (Math|Vector|MakeVector _returnvalue _returnvalue _returnvalue)) "Undefined" 0 0))
                (bind _staticmesh_2 (Variables|/Game/Blueprints/ObjectSpawnSelection/SM_ObjectBlueprint.SM_ObjectBlueprint_C|GetStaticMesh _returnvalue_4)
                  (:then
                    (Physics|SetSimulatePhysics _staticmesh_2 true)
                    (if (Variables|Default|GetSpread)
                      (Physics|AddImpulse _staticmesh_2 (Math|Vector|MakeVector (Math|Random|RandomFloatinRange 0.0 (Variables|Default|GetX)) (Math|Random|RandomFloatinRange 0.0 (Variables|Default|GetY)) (Math|Random|RandomFloatinRange 0.0 (Variables|Default|GetZ))) "None" true)
                      (else
                        (Physics|AddImpulse _staticmesh_2 (Math|Vector|MakeVector (Variables|Default|GetX) (Variables|Default|GetY) (Variables|Default|GetZ)) "None" true))))
                  (:else))))))))))